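; BP_RoomManager is a room manager actor that populates its room with enemies and tracks how many remain.
; On BeginPlay it spawns a small random number of BP_Enemy actors at random points inside the SpawnArea component's bounds, adjusting for collisions but always spawning.
; OnEnemyKilled decrements the remaining count and checks for zero, but nothing yet happens when the room is cleared.
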(event `self.ReceiveBeginPlay`
  (bind (_origin _boxextent) (`KismetSystemLibrary.GetComponentBounds` (`self.SpawnArea`)))
  (bind _output_get (set `self.RemainingEnemies` (`KismetMathLibrary.RandomIntegerInRange` 2 4)))
  (for _ (range 1 (+ _output_get 1))
    (`|SpawnActorFromClass` "/Game/TacticalSurvive/Blueprints/BP_Enemy.BP_Enemy_C" (`KismetMathLibrary.MakeTransform` (`KismetMathLibrary.RandomPointInBoundingBox` _origin _boxextent)) "AdjustIfPossibleButAlwaysSpawn" "MultiplyWithRoot" null null)))

(event `OnEnemyKilled`
  (bind _output_get (set `self.RemainingEnemies` (- (`self.RemainingEnemies`) 1)))
  (if (<= _output_get 0)
    _))

(fn `UserConstructionScript`)
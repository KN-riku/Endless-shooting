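; BP_bulletbox is an ammo pickup that grants a small random amount of reserve ammo to BP_TSCharacter on overlap.
; Box overlap adds the amount to TotalAmmo in BP_MyGameInstance, destroys the box, then refreshes the character HUD's bullet icons.
; The cap check and the addition use separate random rolls, so the total can exceed the intended limit of 40.
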(event `self.Box.OnComponentBeginOverlap`
  (params (OverlappedComponent :type "PrimitiveComponent Object Reference") (OtherActor :type "Actor Object Reference") (OtherComp :type "PrimitiveComponent Object Reference") (OtherBodyIndex :type Integer) (bFromSweep :type Boolean) (SweepResult :type "HitResult Structure (by ref)"))
  (bind _asbp_tscharacter (cast `/Game/TacticalSurvive/Blueprints/BP_TSCharacter` OtherActor))
  (bind _asbp_my_game_instance (cast `/Game/TacticalSurvive/Blueprints/BP_MyGameInstance` (`GameplayStatics.GetGameInstance`)))
  (bind _returnvalue (+ (`/Game/TacticalSurvive/Blueprints/BP_MyGameInstance.TotalAmmo` _asbp_my_game_instance) (`KismetMathLibrary.RandomIntegerInRange` 1 7)))
  (if (> _returnvalue 40)
    (set `/Game/TacticalSurvive/Blueprints/BP_MyGameInstance.TotalAmmo` 40 _asbp_my_game_instance)
    (else
      (set `/Game/TacticalSurvive/Blueprints/BP_MyGameInstance.TotalAmmo` _returnvalue _asbp_my_game_instance)))
  (`self.K2_DestroyActor`)
  (`/Game/TacticalSurvive/Map/UI/WBP_PlayerHUD.UpdateBulletIcons` (`/Game/TacticalSurvive/Blueprints/BP_TSCharacter.HUDRef` _asbp_tscharacter) (`/Game/TacticalSurvive/Blueprints/BP_MyGameInstance.CurrentAmmo` _asbp_my_game_instance) (`/Game/TacticalSurvive/Blueprints/BP_MyGameInstance.TotalAmmo` _asbp_my_game_instance)))

(fn `UserConstructionScript`)